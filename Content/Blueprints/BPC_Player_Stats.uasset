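; Player stats component that tracks health, stamina, XP and level for BP_ThirdPersonCharacter.
; On BeginPlay it waits a tick, caches the owning character and fills its HUD widget.
; Functions change current or max values and push them straight to HUD bars and text, with the decrease functions returning whether the stat is depleted.
; Reaching max XP levels up, resetting XP, raising the threshold and playing sounds.
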(event `self.ReceiveBeginPlay`
  (bind _hud_widget (`/Game/ThirdPerson/Blueprints/BP_ThirdPersonCharacter.HUD Widget` (`self.Player Character BP`)))
  (bind _hud_widget_2 (`/Game/ThirdPerson/Blueprints/BP_ThirdPersonCharacter.HUD Widget` (`self.Player Character BP`)))
  (`KismetSystemLibrary.DelayUntilNextTick`)
  (bind _asbp_third_person_character (cast `/Game/ThirdPerson/Blueprints/BP_ThirdPersonCharacter` (`self.GetOwner`)))
  (set `self.Player Character BP` _asbp_third_person_character)
  (`ProgressBar.SetPercent` (`/Game/UI/WB_HUD.StaminaBar` (`/Game/ThirdPerson/Blueprints/BP_ThirdPersonCharacter.HUD Widget` (`self.Player Character BP`))) (/ (`self.CurrentStamina`) (`self.MaxStamina`)))
  (`ProgressBar.SetPercent` (`/Game/UI/WB_HUD.HealthBar` _hud_widget) (/ (`self.CurrentHealth`) (`self.MaxHealth`)))
  (`TextBlock.SetText` (`/Game/UI/WB_HUD.HealthText` _hud_widget) (`KismetTextLibrary.Conv_DoubleToText` (`self.CurrentHealth`) "HalfToEven"))
  (`ProgressBar.SetPercent` (`/Game/UI/WB_HUD.XPBar` _hud_widget_2) (/ (`self.XP`) (`self.MaxXP`)))
  (`TextBlock.SetText` (`/Game/UI/WB_HUD.XPText` _hud_widget_2) (`|FormatText` "{Current XP}/{Max XP}" (`self.XP`) (`self.MaxXP`)))
  (`TextBlock.SetText` (`/Game/UI/WB_HUD.LevelText` (`/Game/ThirdPerson/Blueprints/BP_ThirdPersonCharacter.HUD Widget` (`self.Player Character BP`))) (`KismetTextLibrary.Conv_IntToText` (`self.Level`))))

(fn `Decrease Health`
  (params (Damage :type "Float (double-precision)"))
  (returns (`Is Player Dead?` :type Boolean))
  (bind _hud_widget (`/Game/ThirdPerson/Blueprints/BP_ThirdPersonCharacter.HUD Widget` (`self.Player Character BP`)))
  (if (not (<= (`self.CurrentHealth`) 0.0))
    (bind _output_get (set `self.CurrentHealth` (- (`self.CurrentHealth`) Damage)))
    (`ProgressBar.SetPercent` (`/Game/UI/WB_HUD.HealthBar` _hud_widget) (/ _output_get (`self.MaxHealth`)))
    (`TextBlock.SetText` (`/Game/UI/WB_HUD.HealthText` _hud_widget) (`KismetTextLibrary.Conv_DoubleToText` (`self.CurrentHealth`) "HalfToEven"))
    (if (<= (`self.CurrentHealth`) 0.0)
      _
      (else
        (return false))))
  (return true))

(fn `Decrease Stamina`
  (params (`Stamina Depleted` :type "Float (double-precision)"))
  (returns (`Not Stamina Left` :type Boolean))
  (bind _hud_widget (`/Game/ThirdPerson/Blueprints/BP_ThirdPersonCharacter.HUD Widget` (`self.Player Character BP`)))
  (if (not (<= (`self.CurrentStamina`) 0.0))
    (set `self.CurrentStamina` (- (`self.CurrentStamina`) `Stamina Depleted`))
    (`ProgressBar.SetPercent` (`/Game/UI/WB_HUD.StaminaBar` _hud_widget) (/ (`self.CurrentStamina`) (`self.MaxStamina`)))
    (`TextBlock.SetText` (`/Game/UI/WB_HUD.StaminaText` _hud_widget) (`KismetTextLibrary.Conv_DoubleToText` (`self.CurrentStamina`) "HalfToEven"))
    (if (<= (`self.CurrentStamina`) 0.0)
      _
      (else
        (return false))))
  (return true))

(fn `Increase Health`
  (params (`Added Health` :type "Float (double-precision)"))
  (bind _hud_widget (`/Game/ThirdPerson/Blueprints/BP_ThirdPersonCharacter.HUD Widget` (`self.Player Character BP`)))
  (set `self.CurrentHealth` (+ (`self.CurrentHealth`) `Added Health`))
  (if (> (`self.CurrentHealth`) (`self.MaxHealth`))
    (set `self.CurrentHealth` (`self.MaxHealth`)))
  (`ProgressBar.SetPercent` (`/Game/UI/WB_HUD.HealthBar` _hud_widget) (/ (`self.CurrentHealth`) (`self.MaxStamina`)))
  (`TextBlock.SetText` (`/Game/UI/WB_HUD.HealthText` _hud_widget) (`KismetTextLibrary.Conv_DoubleToText` (`self.CurrentHealth`) "HalfToEven")))

(fn `Increase level`
  (params (`Added level` :type Integer))
  (set `self.Level` (+ (`self.Level`) `Added level`))
  (set `self.MaxXP` (+ (`self.MaxXP`) 150.0))
  (set `self.XP` 0.0)
  (`TextBlock.SetText` (`/Game/UI/WB_HUD.LevelText` (`/Game/ThirdPerson/Blueprints/BP_ThirdPersonCharacter.HUD Widget` (`self.Player Character BP`))) (`KismetTextLibrary.Conv_IntToText` (`self.Level`)))
  (`GameplayStatics.PlaySound2D` "/Game/Audio/UI/475889__epicsoundeffects__ese-whoosh-epic-level-up.475889__epicsoundeffects__ese-whoosh-epic-level-up" 1.0 1.0 0.0 null null)
  (`GameplayStatics.PlaySound2D` "/Game/Audio/UI/542825__kostas17__magic-spell.542825__kostas17__magic-spell" 1.0 1.0 0.0 null null))

(fn `Increase Max Health`
  (params (`IHealth incremention` :type "Float (double-precision)"))
  (bind _hud_widget (`/Game/ThirdPerson/Blueprints/BP_ThirdPersonCharacter.HUD Widget` (`self.Player Character BP`)))
  (set `self.MaxHealth` (+ (`self.MaxHealth`) `IHealth incremention`))
  (`ProgressBar.SetPercent` (`/Game/UI/WB_HUD.HealthBar` _hud_widget) (/ (`self.CurrentHealth`) (`self.MaxStamina`)))
  (`TextBlock.SetText` (`/Game/UI/WB_HUD.HealthText` _hud_widget) (`KismetTextLibrary.Conv_DoubleToText` (`self.CurrentHealth`) "HalfToEven")))

(fn `Increase Max Stamina`
  (params (`Added Stamina` :type "Float (double-precision)"))
  (set `self.MaxStamina` (+ (`self.MaxStamina`) `Added Stamina`))
  (`ProgressBar.SetPercent` (`/Game/UI/WB_HUD.StaminaBar` (`/Game/ThirdPerson/Blueprints/BP_ThirdPersonCharacter.HUD Widget` (`self.Player Character BP`))) (/ (`self.CurrentStamina`) (`self.MaxStamina`))))

(fn `Increase Stamina`
  (params (`Added Stamina` :type "Float (double-precision)"))
  (bind _maxstamina (`self.MaxStamina`))
  (set `self.CurrentStamina` (+ (`self.CurrentStamina`) `Added Stamina`))
  (`ProgressBar.SetPercent` (`/Game/UI/WB_HUD.StaminaBar` (`/Game/ThirdPerson/Blueprints/BP_ThirdPersonCharacter.HUD Widget` (`self.Player Character BP`))) (/ (`self.CurrentStamina`) (`self.MaxStamina`) 0.0))
  (if (> (`self.CurrentStamina`) _maxstamina)
    (set `self.CurrentStamina` _maxstamina)))

(fn `Increase XP`
  (params (`Added XP` :type "Float (double-precision)"))
  (bind _hud_widget (`/Game/ThirdPerson/Blueprints/BP_ThirdPersonCharacter.HUD Widget` (`self.Player Character BP`)))
  (set `self.XP` (+ (`self.XP`) `Added XP`))
  (if (>= (`self.XP`) (`self.MaxXP`))
    (`self.Increase level` 1))
  (`ProgressBar.SetPercent` (`/Game/UI/WB_HUD.XPBar` _hud_widget) (/ (`self.XP`) (`self.MaxXP`)))
  (`TextBlock.SetText` (`/Game/UI/WB_HUD.XPText` _hud_widget) (`|FormatText` "{Current XP}/{Max XP}" (`self.XP`) (`self.MaxXP`))))